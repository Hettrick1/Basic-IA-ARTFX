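; Player controller that turns Enhanced Input actions into movement, camera look and shooting for the controlled pawn.
; On possess it adds the IMC_Character mapping context to the local player's input subsystem.
; Move input is relative to the control rotation with pitch zeroed, and look input supports an InvertCamera option for pitch.
; Shoot casts the pawn to BP_Player and calls its Shoot with zero start and end vectors.
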(event Input|EnhancedActionEvents|EnhancedInputActionIA_Move
  (params (ActionValue :type Vector%202D%20Structure) (ElapsedSeconds :type Float%20%28double-precision%29) (TriggeredSeconds :type Float%20%28double-precision%29) (InputAction :type Input%20Action%20Object%20Reference :default "/Game/_managers/InGame/Inputs/IA_Move.IA_Move"))
  (bind (_x _y) (Math|Vector2D|BreakVector2D ActionValue))
  (bind _returnvalue (Pawn|GetControlRotation :!class /Script/Engine.Controller))
  (bind _returnvalue_2 (Math|Rotator|MakeRotator (.roll _returnvalue) 0.0 (.yaw _returnvalue)))
  (Pawn|Input|AddMovementInput (Pawn|GetControlledPawn) (Math|Vector|GetForwardVector _returnvalue_2) _y false) ; forward
  (Pawn|Input|AddMovementInput (Pawn|GetControlledPawn) (Math|Vector|GetRightVector _returnvalue_2) _x false) ; right
)

(event Input|EnhancedActionEvents|EnhancedInputActionIA_Look
  (params (ActionValue :type Vector%202D%20Structure) (ElapsedSeconds :type Float%20%28double-precision%29) (TriggeredSeconds :type Float%20%28double-precision%29) (InputAction :type Input%20Action%20Object%20Reference :default "/Game/_managers/InGame/Inputs/IA_Look.IA_Look"))
  (bind (_x _y) (Math|Vector2D|BreakVector2D ActionValue))
  (Class|PlayerController|AddYawInput _x)
  (Class|PlayerController|AddPitchInput (* _y (Math|Float|SelectFloat 1.0 -1.0 (Variables|Default|GetInvert%20Camera)))))

(event Input|EnhancedActionEvents|EnhancedInputActionIA_Shoot
  (params (ActionValue :type Boolean) (ElapsedSeconds :type Float%20%28double-precision%29) (TriggeredSeconds :type Float%20%28double-precision%29) (InputAction :type Input%20Action%20Object%20Reference :default "/Game/_managers/InGame/Inputs/IA_Shoot.IA_Shoot"))
  (:Started
    (bind _asbp_player (Utilities|Casting|CastToBP_Player (Pawn|GetControlledPawn)))
    (Default|Shoot _asbp_player "0, 0, 0" "0, 0, 0")))

(event EventPossess
  (params (PossessedPawn :type Pawn%20Object%20Reference))
  (bind _returnvalue (PlayerController|LocalPlayerSubsystems|GetEnhancedInputLocalPlayerSubsystem))
  (Utilities|IsValid _returnvalue
    (:Is%20Valid
      (Input|AddMappingContext _returnvalue "/Game/_managers/InGame/Inputs/IMC_Character.IMC_Character" 0 "(bIgnoreAllPressedKeysUntilRelease=True,bForceImmediately=False,bNotifyUserSettings=False)"))))

(fn ConstructionScript)