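; Player character Blueprint that shoots from the camera and directs an AI ally toward whatever the shot hits.
; BeginPlay caches the BP_Ally actor found in the level.
; Shoot passes a camera-origin line along control rotation, plus the ally, to the parent implementation.
; On a blocking hit, it writes the hit actor into the ally AI controller's blackboard as the target.
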(event EventBeginPlay
  (bind _returnvalue (Actor|GetActorOfClass "/Game/Characters/BP_Ally.BP_Ally_C"))
  (Variables|Default|SetAllyRef _returnvalue))

(event EventShoot
  (params (Start :type Vector :default "0, 0, 0") (End :type Vector :default "0, 0, 0") ([0] :type Actor%20Object%20Reference))
  (bind _returnvalue (Game|GetPlayerCameraManager 0))
  (bind _shoothit (Variables|Default|GetShootHit))
  (bind (_bblockinghit _binitialoverlap _time _distance _location _impactpoint _normal _impactnormal _physmat _hitactor) (Collision|BreakHitResult _shoothit))
  (bind _returnvalue_2 (Transformation|GetActorLocation _returnvalue))
  (|CallParentFunction _returnvalue_2 (+ _returnvalue_2 (* (Math|Vector|GetForwardVector (Pawn|GetControlRotation :!class /Script/Engine.Pawn)) (Variables|Default|GetShootRange))) (Variables|Default|GetAllyRef))
  (if _bblockinghit
    (AI|Components|Blackboard|SetValueasObject (AI|GetBlackboard (AI|GetAIController (Variables|Default|GetAllyRef))) (Variables|Default|GetTargetRefKey) _hitactor)))

(fn ConstructionScript
  (|CallParentFunction))